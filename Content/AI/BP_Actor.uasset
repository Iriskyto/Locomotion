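; BP_Actor is an actor meant to spawn a configurable actor class at random points around itself.
; BeginPlay gathers five point components into PointArray and does nothing further.
; A self-repeating spawn loop picks a random point's world location, spawns there with collision adjustment, then waits a random few seconds.
; That loop is not connected to any event, so nothing spawns as the graph stands.
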(event EventBeginPlay
  (Variables|Default|SetPointArray (Utilities|Array|MakeArray (Variables|Default|GetPoint1) (Variables|Default|GetPoint2) (Variables|Default|GetPoint3) (Variables|Default|GetPoint4) (Variables|Default|GetPoint5))))

(fn ConstructionScript)