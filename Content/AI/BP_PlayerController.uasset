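; Player controller that lets the player take control of another pawn by looking at it and pressing K.
; The key press fires a visibility line trace from the controlled pawn's location along the control rotation for a short fixed range, ignoring that pawn and drawing debug lines.
; If the hit actor is a Pawn, the controller possesses it.
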(event Input|KeyboardEvents|K
  (params (Key :type Key%20Structure :default "None"))
  (bind _returnvalue (Pawn|GetControlledPawn))
  (bind _returnvalue_2 (Transformation|GetActorLocation _returnvalue))
  (:Pressed
    (bind (_outhit _returnvalue_3) (Collision|LineTraceByChannel _returnvalue_2 (+ _returnvalue_2 (* (Math|Vector|GetForwardVector (Pawn|GetControlRotation :!class /Script/Engine.Controller)) 1e+03)) "TraceTypeQuery1" false (Utilities|Array|MakeArray _returnvalue) "ForDuration"))
    (if _returnvalue_3
      (bind _aspawn (Utilities|Casting|CastToPawn (.HitActor (Collision|BreakHitResult _outhit))))
      (Pawn|Possess _aspawn))))

(fn ConstructionScript)